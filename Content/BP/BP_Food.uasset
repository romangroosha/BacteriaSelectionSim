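; BP_Food is a food pickup actor that simple cells consume on contact.
; On BeginPlay it assigns itself a random food value.
; When an overlapping actor is a BP_SimpleCell or a subclass, it passes itself to that cell through the INTFoodableMessage interface call, leaving the response to the cell.
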(event EventBeginPlay
  (Variables|Default|SetFoodValue (Math|Random|RandomIntegerinRange 10 20)))

(event Collision|EventActorBeginOverlap
  (params (OtherActor :type Actor%20Object%20Reference))
  (if (or (== (Utilities|GetClass OtherActor) "/Game/BP/Cells/BP_SimpleCell.BP_SimpleCell_C") (Utilities|ClassIsChildOf (Utilities|GetClass OtherActor) "/Game/BP/Cells/BP_SimpleCell.BP_SimpleCell_C"))
    (Class|BPIFoodable|INTFoodable(Message) OtherActor self)))

(fn ConstructionScript)