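; BP_SimpleCell_Child is a child cell Blueprint that starts with randomized variations of inherited traits.
; On BeginPlay it runs the parent logic, applies the red cell material to InSide, then calls SetStartingVariables.
; That override randomizes velocity, energy and rotation rate within small ranges around inherited values, and picks a random yaw.
; It prints the inherited energy and leaves the parent's SetStartingVariables unexecuted.
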(event EventBeginPlay
  (|CallParentFunction)
  (Rendering|Material|SetMaterial (Variables|Default|GetInSide) 0 "/Game/Materials/MI_RedCell.MI_RedCell")
  (CallFunction|SetStartingVariables))

(event Collision|EventActorBeginOverlap
  (params (OtherActor :type Actor%20Object%20Reference)))

(event EventTick
  (params (DeltaSeconds :type Float%20%28single-precision%29))
  (|CallParentFunction DeltaSeconds) ; This node is disabled and will not be called.\nDrag off pins to build functionality.
)

(fn ConstructionScript
  (|CallParentFunction))

(fn SetStartingVariables
  (bind _inheritedvelocity (Variables|Default|GetInheritedVelocity))
  (bind _inheritedenergy (Variables|Default|GetInheritedEnergy))
  (bind _inheritedrotrate (Variables|Default|GetInheritedRotRate))
  (Variables|Default|SetVelocity (Math|Random|RandomFloatinRange (- _inheritedvelocity 1.0) (+ _inheritedvelocity 1.0)))
  (Variables|Default|SetEnergy (Math|Random|RandomFloatinRange (- _inheritedenergy 1.0) (+ _inheritedenergy 1.0)))
  (Variables|Default|SetRotationRate (Math|Random|RandomFloatinRange (- _inheritedrotrate 5.0) (+ _inheritedrotrate 5.0)))
  (Transformation|SetActorRotation (Math|Rotator|MakeRotator 0.0 0.0 (Math|Random|RandomFloatinRange 0.0 3.6e+02)))
  (Development|PrintString (Utilities|String|ToString(Float) (Variables|Default|GetInheritedEnergy))))