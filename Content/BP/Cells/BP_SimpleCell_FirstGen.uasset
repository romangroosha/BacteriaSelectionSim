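; BP_SimpleCell_FirstGen is a child cell Blueprint that gives first-generation cells randomized starting traits.
; Its construction script runs the parent's script, then calls SetStartingVariables.
; That override replaces the parent version, randomizing velocity, energy, rotation rate and yaw, and saving the rolled energy as StartingEnergy.
; The event graph adds no logic of its own, leaving runtime behavior to the parent class.
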(event EventBeginPlay
  (|CallParentFunction))

(event Collision|EventActorBeginOverlap
  (params (OtherActor :type Actor%20Object%20Reference)))

(event EventTick
  (params (DeltaSeconds :type Float%20%28single-precision%29))
  (|CallParentFunction DeltaSeconds) ; This node is disabled and will not be called.\nDrag off pins to build functionality.
)

(fn ConstructionScript
  (|CallParentFunction)
  (CallFunction|SetStartingVariables))

(fn SetStartingVariables
  (Variables|Default|SetVelocity (Math|Random|RandomFloatinRange 2.0 3e+01))
  (bind _output_get (Variables|Default|SetEnergy (Math|Random|RandomFloatinRange 6e+01 9e+01)))
  (Variables|Default|SetStartingEnergy _output_get)
  (Variables|Default|SetRotationRate (Math|Random|RandomFloatinRange 3e+01 1.8e+02))
  (Transformation|SetActorRotation (Math|Rotator|MakeRotator 0.0 0.0 (Math|Random|RandomFloatinRange 0.0 3.6e+02))))