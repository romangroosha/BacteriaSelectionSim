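; BP_SimpleCell is a simulated cell that wanders, eats, reproduces and dies, updating the game mode's cell total.
; A timeline lerps it to random nearby locations and yaws, while Tick drains energy by velocity and food restores it.
; A timed check spends surplus energy to spawn offspring inheriting its traits.
; Exhaustion or a second birth destroys it, scattering food; clicking it makes the camera follow.
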(event OnComponentBeginOverlap(FrontSide)
  (params (OverlappedComponent :type Primitive%20Component%20Object%20Reference) (OtherActor :type Actor%20Object%20Reference) (OtherComp :type Primitive%20Component%20Object%20Reference) (OtherBodyIndex :type Integer) (bFromSweep :type Boolean) (SweepResult :type Hit%20Result%20Structure%20%28by%20ref%29))
  ;[1 0.2993 0] Fix that
)

(event Custom|RotationTick
  ;[1 1 1] Rotation
  (CallFunction|RandomTargetAcotorLoc 1e+01)
  (CallFunction|FindTargetRotatiot)
  (bind _0_to_1__0_5s_ (Timeline|MoveAndRotate PlayFromStart)
    (:Update
      (Transformation|SetActorLocation (Math|Vector|Lerp(Vector) (Variables|Default|GetCurrentActorLoc_BA) (Variables|Default|GetTargetActorLoc_BA) _0_to_1__0_5s_) false false)
      (Transformation|SetActorRotation (Math|Rotator|Lerp(Rotator) (Variables|Default|GetCurrentActorRot_BA) (Variables|Default|GetTargetActorRot_BA) _0_to_1__0_5s_ true)))))

(event Custom|PreDeath
  ;[1 1 1] Pre Death Actions
  (Actor|Tick|SetActorTickEnabled false)
  (Variables|/Script/Engine.PrimitiveComponent|SetbGenerateOverlapEvents (Variables|Default|GetFrontSide) false)
  (CallFunction|ChangeCellTotal -1)
  (for _index (range 0 10)
    (CallFunction|SpawnFoodAfterDeath 200))
  (for _index_2 (range 0 20)
    (CallFunction|SpawnFoodAfterDeath 600))
  (Actor|DestroyActor))

(event Custom|Birth
  (if (and (>= (Variables|Default|GetEnergy) 1e+02) (<= (Variables|Default|GetEnergy) 1.5e+02)) ; should make a birth?
    (Utilities|FlowControl|DoOnce false :!label _label
      (:Completed
        (Variables|Default|SetEnergy (- (Variables|Default|GetEnergy) 5e+01))
        (Math|Integer|IncrementInt (Variables|Default|GetBirthCounter)
          (:%20%20
            (bind _returnvalue (Game|SpawnActorfromClass "/Game/BP/Cells/BP_SimpleCell_Offspring.BP_SimpleCell_Offspring_C" (Transformation|GetActorTransform) "AdjustIfPossibleButAlwaysSpawn" 0 0))
            (Variables|/Game/BP/Cells/BP_SimpleCell_Offspring.BP_SimpleCell_Offspring_C|SetInheritedVelocity _returnvalue (Variables|Default|GetVelocity))
            (Variables|/Game/BP/Cells/BP_SimpleCell_Offspring.BP_SimpleCell_Offspring_C|SetInheritedEnergy _returnvalue (Variables|Default|GetStartingEnergy))
            (Variables|/Game/BP/Cells/BP_SimpleCell_Offspring.BP_SimpleCell_Offspring_C|SetInheritedRotRate _returnvalue (Variables|Default|GetRotationRate))
            (CallFunction|ChangeCellTotal 1)
            (if (>= (Variables|Default|GetBirthCounter) 2)
              (CallFunction|PreDeath)
              (else
                (Utilities|FlowControl|Delay 1e+01)
                (goto _label Reset)))))))))

(event EventBeginPlay
  (Utilities|Time|SetTimerbyEvent (EventDispatchers|CreateEvent :!event Custom|RotationTick) 0.5 true 0.1 0.5)
  (Utilities|Time|SetTimerbyFunctionName 0 "Birth" 5.0 true 0.1 0.5) ; Check for time to birth
)

(event MouseInput|EventActorOnClicked
  (params (ButtonPressed :type Key%20Structure :default "None"))
  ;[1 1 1] Follow Camera
  (bind _asbp_camera (Utilities|Casting|CastToBP_Camera (Game|GetPlayerCharacter 0)))
  (Variables|/Game/BP/BP_Camera.BP_Camera_C|SetFollowActor _asbp_camera self))

(event EventTick
  (params (DeltaSeconds :type Float%20%28single-precision%29))
  (if (<= (Variables|Default|GetEnergy) 0.0) ; if should die
    (CallFunction|PreDeath)
    (else
      (CallFunction|Energy-Velocity 5e+02)
      (CallFunction|ParamstoText))))

(event EventINTFoodable
  (params (BP_Food :type BP%20Food%20Object%20Reference))
  ;[1 1 1] Food
  (CallFunction|EatFood BP_Food))

(fn ConstructionScript)

(fn SpawnFoodAfterDeath
  (params (SpawnRange :type Integer))
  (bind _returnvalue (Transformation|GetActorLocation))
  (bind _returnvalue_2 (* SpawnRange -1))
  (Game|SpawnActorfromClass "/Game/BP/BP_FoodAfterDeath.BP_FoodAfterDeath_C" (Math|Transform|MakeTransform (Math|Vector|MakeVector (+ (.x _returnvalue) (Math|Random|RandomIntegerinRange _returnvalue_2 SpawnRange)) (+ (.y _returnvalue) (Math|Random|RandomIntegerinRange _returnvalue_2 SpawnRange)) 0.0) "0, 0, 0" "1.000000,1.000000,1.000000") "AdjustIfPossibleButAlwaysSpawn" 0 0))

(fn Energy-Velocity
  (params (Coef :type Float%20%28double-precision%29))
  (Variables|Default|SetEnergy (- (Variables|Default|GetEnergy) (/ (Variables|Default|GetVelocity) Coef))))

(fn ParamstoText
  (Rendering|Components|TextRender|SetText (Variables|Default|GetTextEnergy) (Utilities|Text|ToText(Integer) (Math|Float|Truncate (Variables|Default|GetEnergy))))
  (Rendering|Components|TextRender|SetText (Variables|Default|GetTextVelocity) (Utilities|Text|ToText(Integer) (Math|Float|Truncate (Variables|Default|GetVelocity))))
  (Rendering|Components|TextRender|SetText (Variables|Default|GetTextRotRate) (Utilities|Text|ToText(Integer) (Math|Float|Truncate (Variables|Default|GetRotationRate)))))

(fn ChangeLocationOld
  (params (DeltaTime :type Float%20%28single-precision%29))
  (bind _returnvalue (Transformation|GetActorLocation))
  (Transformation|SetActorLocation (Math|Interpolation|VInterpTo _returnvalue (+ _returnvalue (* (Transformation|GetActorForwardVector) (Variables|Default|GetVelocity))) DeltaTime 0.0) false false))

(fn ChangeRotationOld
  (bind _returnvalue (Transformation|GetActorRotation))
  (Transformation|SetActorRotation (Math|Rotator|MakeRotator 0.0 0.0 (Math|Interpolation|FInterpTo (.yaw _returnvalue) (+ (.yaw _returnvalue) (Math|Random|RandomFloatinRange (Math|Random|RandomFloatinRange (* (Variables|Default|GetRotationRate) -1.0) 0.0) (Math|Random|RandomFloatinRange 0.0 (Variables|Default|GetRotationRate)))) (Utilities|Time|GetWorldDeltaSeconds) 0.0))))

(fn SetStartingVariables
  (Variables|Default|SetVelocity (Math|Random|RandomFloatinRange 2.0 15.0))
  (bind _output_get (Variables|Default|SetEnergy (Math|Random|RandomFloatinRange 5e+01 7e+01)))
  (Variables|Default|SetStartingEnergy _output_get)
  (Variables|Default|SetRotationRate (Math|Random|RandomFloatinRange 3e+01 1.8e+02))
  (Transformation|SetActorRotation (Math|Rotator|MakeRotator 0.0 0.0 (Math|Random|RandomFloatinRange 0.0 3.6e+02))))

(fn AddMovement
  (params (Delta :type Float%20%28double-precision%29))
  (Pawn|Input|AddMovementInput (Transformation|GetActorForwardVector) (* (* Delta 5.0) (Variables|Default|GetVelocity)) false))

(fn ChangeRotation
  (params (DeltaTime :type Float%20%28double-precision%29))
  (Transformation|SetActorRotation (Math|Rotator|MakeRotator 0.0 0.0 (Math|Interpolation|FInterpTo (.yaw (Transformation|GetActorRotation)) (Variables|Old|GetTargetRotation) DeltaTime 5.0))))

(fn FindTargetRotationFloat
  (bind _rotationrate (Variables|Default|GetRotationRate))
  (Variables|Old|SetTargetRotation (+ (.yaw (Transformation|GetActorRotation)) (Math|Random|RandomFloatinRange (* _rotationrate -1.0) _rotationrate))))

(fn EatFood
  (params (Food%20Actor :type BP%20Food%20Object%20Reference))
  (if (<= (Variables|Default|GetEnergy) 1.5e+02)
    (Utilities|IsValid Food%20Actor
      (:Is%20Valid
        (Variables|Default|SetEnergy (+ (Variables|Default|GetEnergy) (Variables|/Game/BP/BP_Food.BP_Food_C|GetFoodValue Food%20Actor)))
        (Actor|DestroyActor Food%20Actor)))))

(fn ChangeCellTotal
  (params (Int :type Integer))
  (bind _asbp_game_mode (Utilities|Casting|CastToBP_GameMode (Game|GetGameMode)))
  (Variables|/Game/BP/BP_GameMode.BP_GameMode_C|SetTotalSimpleCells _asbp_game_mode (+ (Variables|/Game/BP/BP_GameMode.BP_GameMode_C|GetTotalSimpleCells _asbp_game_mode) Int)))

(fn RandomTargetAcotorLoc
  (params (Coef :type Float%20%28double-precision%29))
  (LocalVariables|SetCoef_Local Coef)
  (Variables|Default|SetCurrentActorLoc_BA (Transformation|GetActorLocation))
  (Variables|Default|SetTargetActorLoc_BA (+ (Transformation|GetActorLocation) (Math|Vector|MakeVector (* (Math|Random|RandomFloatinRange (* (LocalVariables|GetCoef_Local) -1.0) (LocalVariables|GetCoef_Local)) (Variables|Default|GetVelocity)) (* (Math|Random|RandomFloatinRange (* (LocalVariables|GetCoef_Local) -1.0) (LocalVariables|GetCoef_Local)) (Variables|Default|GetVelocity)) 0.0)))
  (return))

(fn FindTargetRotatiot
  (bind _returnvalue (Transformation|GetActorRotation))
  (bind _rotationrate (Variables|Default|GetRotationRate))
  (Variables|Default|SetCurrentActorRot_BA (Transformation|GetActorRotation))
  (Variables|Default|SetTargetActorRot_BA (Math|Rotator|MakeRotator (.roll _returnvalue) (.pitch _returnvalue) (+ (.yaw _returnvalue) (Math|Random|RandomFloatinRange (* _rotationrate -1.0) _rotationrate)))))