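; Cell spawner Blueprint meant to scatter a configurable number of cell actors at random positions on a flat square area around itself.
; PreSpawnCells loops over CellAmount, adding a Child Actor Component of CellClass at each relative transform from RandomLocation, which picks whole-number X/Y at zero height.
; The PreSpawnCells call in the Construction Script is disconnected and the event graph is empty, so the Blueprint spawns nothing by itself.
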(event EventBeginPlay)

(event Collision|EventActorBeginOverlap
  (params (OtherActor :type Actor%20Object%20Reference)))

(event EventTick
  (params (DeltaSeconds :type Float%20%28single-precision%29)))

(fn ConstructionScript)

(fn RandomLocation
  (params (Min%20X :type Integer) (Max%20X :type Integer) (Min%20Y :type Integer) (Max%20Y :type Integer))
  (return (Math|Transform|MakeTransform (Math|Vector|MakeVector (Math|Conversions|ToFloat(Integer) (Math|Random|RandomIntegerinRange Min%20X Max%20X)) (Math|Conversions|ToFloat(Integer) (Math|Random|RandomIntegerinRange Min%20Y Max%20Y)) 0.0) "0, 0, 0" "1.000000,1.000000,1.000000")))

(fn PreSpawnCells
  (for _index (range 0 (Variables|Default|GetCell%20Amount))
    (bind _returnvalue (AddComponent|AddChildActorComponent false (CallFunction|RandomLocation -10000 10000 -10000 10000)))
    (ChildActorComponent|SetChildActorClass _returnvalue (Variables|Default|GetCell%20Class))))