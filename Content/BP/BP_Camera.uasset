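; BP_Camera is a movable camera pawn with a spring arm that can pan, zoom and follow an actor.
; While FollowActor is valid, Tick snaps the camera to that actor's X and Y at a fixed height.
; Directional axis inputs add movement along the forward and right vectors at double the axis value.
; The mouse wheel axis adjusts the spring arm length without clamping.
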(event EventBeginPlay)

(event EventTick
  (params (DeltaSeconds :type Float%20%28single-precision%29))
  (bind _followactor (Variables|Default|GetFollowActor))
  (bind _returnvalue (Transformation|GetActorLocation _followactor))
  (Utilities|IsValid _followactor
    (:Is%20Valid
      (Transformation|SetActorLocation (Math|Vector|MakeVector (.x _returnvalue) (.y _returnvalue) 1.5e+02) false false))))

(event Input|AxisEvents|InputAxisAxisUp
  (params (AxisValue :type Float%20%28single-precision%29))
  ;[1 1 1] Move Camera WASD
  (Pawn|Input|AddMovementInput (Transformation|GetActorForwardVector) (+ AxisValue (stale Input|AxisEvents|InputAxisAxisDown AxisValue)) false))

(event Input|AxisEvents|InputAxisAxisDown
  (params (AxisValue :type Float%20%28single-precision%29))
  ;[1 1 1] Move Camera WASD
  (Pawn|Input|AddMovementInput (Transformation|GetActorForwardVector) (+ (stale Input|AxisEvents|InputAxisAxisUp AxisValue) AxisValue) false))

(event Input|AxisEvents|InputAxisAxisRight
  (params (AxisValue :type Float%20%28single-precision%29))
  ;[1 1 1] Move Camera WASD
  (Pawn|Input|AddMovementInput (Transformation|GetActorRightVector) (+ AxisValue (stale Input|AxisEvents|InputAxisAxisLeft AxisValue)) false))

(event Input|AxisEvents|InputAxisAxisLeft
  (params (AxisValue :type Float%20%28single-precision%29))
  ;[1 1 1] Move Camera WASD
  (Pawn|Input|AddMovementInput (Transformation|GetActorRightVector) (+ (stale Input|AxisEvents|InputAxisAxisRight AxisValue) AxisValue) false))

(event Input|AxisEvents|InputAxisMouseWheelAxis
  (params (AxisValue :type Float%20%28single-precision%29))
  ;[1 1 1] Change Camera Disctance with Mouse Wheel
  (Variables|/Script/Engine.SpringArmComponent|SetTargetArmLength (Variables|Default|GetSpringArm) (+ (* AxisValue -3e+02) (Variables|/Script/Engine.SpringArmComponent|GetTargetArmLength (Variables|Default|GetSpringArm)))))

(fn ConstructionScript)