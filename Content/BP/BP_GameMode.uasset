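; Game mode blueprint that sets up the cell count and on-screen GUI when play begins.
; On BeginPlay it finds the BP_CellSpawner in the level through a cached, validity-checked lookup and copies its CellAmount into TotalSimpleCells.
; It then creates a BP_SomeGUI widget and adds it to the viewport, while Tick does nothing.
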(event EventBeginPlay
  (CallFunction|SetBPCellSpawnerRef)
  (Variables|Default|SetTotalSimpleCells (Variables|/Game/BP/BP_CellSpawner.BP_CellSpawner_C|GetCell%20Amount (Variables|Default|GetBP_CellSpawner_Ref)))
  (bind _returnvalue (UserInterface|CreateWidget "/Game/BP/BP_SomeGUI.BP_SomeGUI_C"))
  (UserInterface|Viewport|AddtoViewport _returnvalue 0))

(event EventTick
  (params (DeltaSeconds :type Float%20%28single-precision%29)))

(fn ConstructionScript)

(fn SetBPCellSpawnerRef
  (Utilities|IsValid (Variables|Default|GetBP_CellSpawner_Ref)
    (:Is%20Not%20Valid
      (bind _returnvalue (Actor|GetActorOfClass "/Game/BP/BP_CellSpawner.BP_CellSpawner_C"))
      (Variables|Default|SetBP_CellSpawner_Ref _returnvalue))))